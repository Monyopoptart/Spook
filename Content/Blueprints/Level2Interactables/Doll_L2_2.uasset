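; Level 2 interactable doll actor that shows a one-time WhatIsThisDoll widget when the player presses Interact near it.
; Box overlap shows the PressE prompt and enables input for PlayerCharator, while end overlap hides and disables them through logic shared with BeginPlay.
; An Interacted flag blocks repeat widget creation, and the construction script sets the prompt text from ChangeText.
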(event OnComponentBeginOverlap(Box)
  (params (OverlappedComponent :type Primitive%20Component%20Object%20Reference) (OtherActor :type Actor%20Object%20Reference) (OtherComp :type Primitive%20Component%20Object%20Reference) (OtherBodyIndex :type Integer) (bFromSweep :type Boolean) (SweepResult :type Hit%20Result%20Structure%20%28by%20ref%29))
  (Rendering|SetVisibility (Variables|Default|GetPress%20E) true false)
  (Utilities|Casting|CastToPlayerCharator OtherActor)
  (Input|EnableInput (Game|GetPlayerController 0)))

(event OnComponentEndOverlap(Box)
  (params (OverlappedComponent :type Primitive%20Component%20Object%20Reference) (OtherActor :type Actor%20Object%20Reference) (OtherComp :type Primitive%20Component%20Object%20Reference) (OtherBodyIndex :type Integer))
  (Rendering|SetVisibility (Variables|Default|GetPress%20E) false false)
  (Utilities|Casting|CastToPlayerCharator OtherActor)
  (Input|DisableInput (Game|GetPlayerController 0)))

(event EventBeginPlay
  (Rendering|SetVisibility (Variables|Default|GetPress%20E) false false)
  (Utilities|Casting|CastToPlayerCharator (stale OnComponentEndOverlap(Box) OtherActor))
  (Input|DisableInput (Game|GetPlayerController 0)))

(event Collision|EventActorBeginOverlap
  (params (OtherActor :type Actor%20Object%20Reference)))

(event EventTick
  (params (DeltaSeconds :type Float%20%28single-precision%29)))

(event Input|ActionEvents|InputActionInteract
  (params (Key :type Key%20Structure :default "None"))
  (:Pressed
    (if (not (Variables|Default|GetInteracted))
      (bind _returnvalue (UserInterface|CreateWidget "/Game/UI/InteractiveObjectsHere/WhatIsThisDoll.WhatIsThisDoll_C" (Game|GetPlayerController 0)))
      (UserInterface|Viewport|AddtoViewport _returnvalue 0)
      (Variables|Default|SetInteracted true))))

(fn ConstructionScript
  (Rendering|Components|TextRender|SetText (Variables|Default|GetPress%20E) (Variables|Default|GetChangeText)))