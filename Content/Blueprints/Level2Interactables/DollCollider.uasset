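; DollCollider is a Level 2 puzzle trigger where dolls are brought to unlock a change in the level.
; Its Box overlap counts entering Doll_L2_2 actors after a short delay, capping at two and never decrementing.
; Player overlap toggles a text prompt's visibility.
; If both counts are registered when the player enters, it moves ActorToMove to LocationToMoveActor, changes the text and shows the IThinkIHeardSomething widget.
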(event OnComponentBeginOverlap(Box)
  (params (OverlappedComponent :type Primitive%20Component%20Object%20Reference) (OtherActor :type Actor%20Object%20Reference) (OtherComp :type Primitive%20Component%20Object%20Reference) (OtherBodyIndex :type Integer) (bFromSweep :type Boolean) (SweepResult :type Hit%20Result%20Structure%20%28by%20ref%29))
  (Utilities|FlowControl|Sequence
    (:then_0
      (Utilities|Casting|CastToDoll_L2_2 OtherActor)
      (Utilities|FlowControl|Delay 0.5)
      (if (== (Variables|Default|GetCountDolls) 0)
        (Variables|Default|SetCountDolls 1)
        (else
          (Variables|Default|SetCountDolls 2))))
    (:then_1
      (Utilities|Casting|CastToPlayerCharator OtherActor)
      (Rendering|SetVisibility (Variables|Default|GetTextRender) true false)
      (if (== (Variables|Default|GetCountDolls) 2)
        (Transformation|SetActorLocation (Variables|Default|GetActorToMove) (Variables|Default|GetLocationToMoveActor) false false)
        (bind _output_get (Variables|Default|SetChangeTextRender "All my Children are here"))
        (Rendering|Components|TextRender|SetText (Variables|Default|GetTextRender) _output_get)
        (bind _returnvalue (UserInterface|CreateWidget "/Game/UI/InteractiveObjectsHere/IThinkIHeardSomething.IThinkIHeardSomething_C" (Game|GetPlayerController 0)))
        (UserInterface|Viewport|AddtoViewport _returnvalue 0)))))

(event OnComponentEndOverlap(Box)
  (params (OverlappedComponent :type Primitive%20Component%20Object%20Reference) (OtherActor :type Actor%20Object%20Reference) (OtherComp :type Primitive%20Component%20Object%20Reference) (OtherBodyIndex :type Integer))
  (Utilities|Casting|CastToPlayerCharator OtherActor)
  (Rendering|SetVisibility (Variables|Default|GetTextRender) false false))

(event EventBeginPlay
  (bind _output_get (Variables|Default|SetChangeTextRender "Bring The Dolls Here"))
  (Rendering|Components|TextRender|SetText (Variables|Default|GetTextRender) _output_get)
  (Rendering|SetVisibility (Variables|Default|GetTextRender) false false))

(event Collision|EventActorBeginOverlap
  (params (OtherActor :type Actor%20Object%20Reference)))

(event EventTick
  (params (DeltaSeconds :type Float%20%28single-precision%29)))

(fn ConstructionScript)