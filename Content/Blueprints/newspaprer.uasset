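; Interactable newspaper actor that displays lore text on screen.
; Interact and Activate share one path that creates a Lore widget for the first player controller if none exists, adds it to the viewport and passes in the Lore2 value.
; Hover events are empty, and leftover logic for removing the widget and rotating a scene component toward the player is disconnected.
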(event EventBeginPlay)

(event Collision|EventActorBeginOverlap
  (params (OtherActor :type Actor%20Object%20Reference)))

(event EventTick
  (params (DeltaSeconds :type Float%20%28single-precision%29)))

(event EventActivate
  (Utilities|IsValid (Variables|Default|Gettext)
    (:Is%20Not%20Valid
      (bind _returnvalue (UserInterface|CreateWidget "/Game/UI/lore.lore_C" (Game|GetPlayerController 0)))
      (bind _output_get (Variables|Default|Settext _returnvalue))
      (UserInterface|Viewport|AddtoViewport _output_get 0)
      (Variables|/Game/UI/lore.lore_C|Setlore1 (Variables|Default|Gettext) (Variables|Default|Getlore2)))))

(event EventUnHover)

(event EventHover)

(event EventInteract
  (params (Interactor :type Actor%20Object%20Reference))
  (Utilities|IsValid (Variables|Default|Gettext)
    (:Is%20Not%20Valid
      (bind _returnvalue (UserInterface|CreateWidget "/Game/UI/lore.lore_C" (Game|GetPlayerController 0)))
      (bind _output_get (Variables|Default|Settext _returnvalue))
      (UserInterface|Viewport|AddtoViewport _output_get 0)
      (Variables|/Game/UI/lore.lore_C|Setlore1 (Variables|Default|Gettext) (Variables|Default|Getlore2)))))

(fn ConstructionScript)