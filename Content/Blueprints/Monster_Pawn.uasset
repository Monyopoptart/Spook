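; Monster pawn that wanders around its spawn point using navmesh movement.
; Each tick, when CanWander is set, it moves to a random reachable point around that origin and starts a random timer to re-enable wandering, regardless of arrival.
; While PlayerNearby is false, it snaps its yaw to the movement velocity.
; BeginPlay also gives the Body a dynamic material instance.
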(event EventTick
  (params (DeltaSeconds :type Float%20%28single-precision%29))
  (bind _floatingpawnmovement (Variables|Default|GetFloatingPawnMovement))
  (bind _velocity (Variables|/Script/Engine.MovementComponent|GetVelocity _floatingpawnmovement))
  (Utilities|FlowControl|Sequence
    (:then_0
      (CallFunction|WandertoPoint))
    (:then_1
      (if (not (Variables|Default|GetPlayerNearby))
        (if (> (Math|Vector|VectorLengthSquared _velocity) 0.1)
          (Transformation|SetActorRotation (Math|Rotator|MakeRotator 0.0 0.0 (.yaw (Math|Rotator|MakeRotfromX _velocity)))))))))

(event EventBeginPlay
  (bind _returnvalue (Transformation|GetActorLocation))
  (bind _returnvalue_2 (Rendering|Material|CreateDynamicMaterialInstance 0 "None" :!class /Script/Engine.KismetMaterialLibrary))
  (bind _output_get (Variables|Default|SetDynamicMaterial _returnvalue_2))
  (Rendering|Material|SetMaterial (Variables|Default|GetBody) 0 _output_get)
  (Variables|Default|SetTargetLocation _returnvalue)
  (Variables|Default|SetWanderCenter _returnvalue))

(fn ConstructionScript)

(fn WandertoPoint
  (if (Variables|Default|GetCanWander)
    (if true
      (Variables|Default|SetCanWander false)
      (Utilities|Time|SetTimerbyFunctionName 0 "SetCanWander" (Math|Random|RandomFloatinRange 0.0 1.5))
      (Variables|Default|SetTargetLocation (.RandomLocation (AI|Navigation|GetRandomReachablePointinRadius (Variables|Default|GetWanderCenter) 5e+02 0 0)))
      (AI|Navigation|SimpleMovetoLocation (Pawn|GetController) (Variables|Default|GetTargetLocation)))))

(fn SetCanWander
  (Variables|Default|SetCanWander true))