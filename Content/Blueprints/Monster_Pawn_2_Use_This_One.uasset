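; Monster pawn that wanders the navmesh at random, chases the player on sight and applies damage on capsule overlap.
; PawnSensing sets a sight flag and starts an AI move toward the player, with a delay later clearing the flag.
; Tick snaps yaw toward the current target and either re-enters the chase logic or, after a delay, picks another nearby random point.
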(event OnSeePawn(PawnSensing)
  (params (Pawn :type Pawn%20Object%20Reference))
  ;[1 1 1] Player is in sight
  (Variables|Default|SetIsPlayerInSight true)
  (bind _asplayer_charator (Utilities|Casting|CastToPlayerCharator Pawn))
  (Variables|Default|SetLocationToRotateTo (.yaw (Math|Rotator|FindLookatRotation (Transformation|GetActorLocation) (Transformation|GetActorLocation Pawn))))
  (AI|AIMoveTo self "0, 0, 0" _asplayer_charator 5.0 false
    (:then
      (Utilities|FlowControl|Delay 5.0)
      (Variables|Default|SetIsPlayerInSight false))))

(event OnComponentBeginOverlap(Capsule)
  (params (OverlappedComponent :type Primitive%20Component%20Object%20Reference) (OtherActor :type Actor%20Object%20Reference) (OtherComp :type Primitive%20Component%20Object%20Reference) (OtherBodyIndex :type Integer) (bFromSweep :type Boolean) (SweepResult :type Hit%20Result%20Structure%20%28by%20ref%29))
  (bind _asplayer_charator (Utilities|Casting|CastToPlayerCharator OtherActor))
  (Game|Damage|ApplyDamage _asplayer_charator (Variables|Default|GetDamage) 0 0))

(event Custom|MoveToRandomPoint
  (bind _returnvalue (Transformation|GetActorLocation))
  ;[1 1 1] Random Wander
  (Variables|Default|SetRandomPoint (.RandomLocation (Class|NavigationSystemV1|GetRandomPointinNavigableRadius _returnvalue 1e+03 0 0)))
  (Variables|Default|SetLocationToRotateTo (.yaw (Math|Rotator|FindLookatRotation _returnvalue (Variables|Default|GetRandomPoint))))
  (AI|AIMoveTo self (Variables|Default|GetRandomPoint) 0 5.0 false))

(event Custom|PlayerIsInSight
  ;[1 1 1] Player is in sight
  (bind _asplayer_charator (Utilities|Casting|CastToPlayerCharator (stale OnSeePawn(PawnSensing) Pawn)))
  (Variables|Default|SetLocationToRotateTo (.yaw (Math|Rotator|FindLookatRotation (Transformation|GetActorLocation) (Transformation|GetActorLocation (stale OnSeePawn(PawnSensing) Pawn)))))
  (AI|AIMoveTo self "0, 0, 0" _asplayer_charator 5.0 false
    (:then
      (Utilities|FlowControl|Delay 5.0)
      (Variables|Default|SetIsPlayerInSight false))))

(event EventTick
  (params (DeltaSeconds :type Float%20%28single-precision%29))
  ;[1 1 1] Runs all the time
  (Transformation|SetActorRotation (Math|Rotator|MakeRotator 0.0 0.0 (Variables|Default|GetLocationToRotateTo)))
  (if (Variables|Default|GetIsPlayerInSight)
    (CallFunction|PlayerIsinSight)
    (else
      (Utilities|FlowControl|Delay 2.5)
      (CallFunction|MovetoRandomPoint))))

(event EventBeginPlay
  ;[1 1 1] Runs all the time
  (CallFunction|MovetoRandomPoint))

(fn ConstructionScript)