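; LightningBox is a trigger volume that plays a lightning strike when the player character overlaps its box.
; After a one-second delay it plays a thunder sound at its location, then flashes a RectLight twice through hand-unrolled intensity toggles and delays.
; A CD flag, cleared after the flashes and restored fifteen seconds later, serves as a cooldown.
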(event OnComponentBeginOverlap(Box)
  (params (OverlappedComponent :type Primitive%20Component%20Object%20Reference) (OtherActor :type Actor%20Object%20Reference) (OtherComp :type Primitive%20Component%20Object%20Reference) (OtherBodyIndex :type Integer) (bFromSweep :type Boolean) (SweepResult :type Hit%20Result%20Structure%20%28by%20ref%29))
  ;[1 1 1] Code by Eric
  (Utilities|Casting|CastToPlayerCharator OtherActor)
  (if (Variables|Default|GetCD)
    (Utilities|FlowControl|Delay 1.0)
    (Audio|PlaySoundatLocation "/Game/Audio/475900__mattiagiovanetti__thunder-and-the-bird.475900__mattiagiovanetti__thunder-and-the-bird" (Transformation|GetActorLocation (Components|GetOwner (Variables|Default|GetDefaultSceneRoot))) "0, 0, 0" 2.0 1.0 0.0 0 0 0)
    ;[1 1 1] Repeat as Loop was being fickle
    (Rendering|Components|Light|SetIntensity (Variables|Default|GetRectLight) (Variables|Default|GetIntense))
    (Utilities|FlowControl|Delay 0.2)
    (Rendering|Components|Light|SetIntensity (Variables|Default|GetRectLight) 0.0)
    (Utilities|FlowControl|Delay 0.2)
    (Rendering|Components|Light|SetIntensity (Variables|Default|GetRectLight) (Variables|Default|GetIntense))
    (Utilities|FlowControl|Delay 0.2)
    (Rendering|Components|Light|SetIntensity (Variables|Default|GetRectLight) 0.0)
    (Variables|Default|SetCD false)
    (Utilities|FlowControl|Delay 15.0)
    (Variables|Default|SetCD true)))

(fn ConstructionScript)